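; CheckpointBP is a one-time checkpoint actor that updates the player's saved initial position.
; On BeginPlay it spawns a CheckpointParticleSystemBP at its collision component's location and rotation.
; The first overlap by a Player-tagged BP_ThirdPersonCharacter sets that character's InitialPosition to the checkpoint location plus a spawn offset, marks it checked and plays audio.
; A final LastCheckpoint branch does nothing.
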(event `self.ReceiveBeginPlay`
  (bind (_returnvalue_location _returnvalue_rotation) (`KismetMathLibrary.BreakTransform` (`SceneComponent.K2_GetComponentToWorld` (`self.CollisionComponent`))))
  (`|SpawnActorFromClass` "/Game/Blueprints/CheckpointParticleSystemBP.CheckpointParticleSystemBP_C" (`KismetMathLibrary.MakeTransform` _returnvalue_location _returnvalue_rotation) "AlwaysSpawn" "OverrideRootScale" null null))

(event `self.ReceiveActorBeginOverlap`
  (params (OtherActor :type "Actor Object Reference"))
  (if (`self.ActorHasTag` OtherActor "Player")
    (if (not (`self.Checked`))
      (bind _asbp_third_person_character (cast `/Game/Blueprints/PlayerCharacters/BP_ThirdPersonCharacter` OtherActor))
      (set `/Game/Blueprints/PlayerCharacters/BP_ThirdPersonCharacter.InitialPosition` (+ (`self.K2_GetActorLocation`) (`self.CharacterSpawnOffset`)) _asbp_third_person_character)
      (set `self.Checked` true)
      (`AudioComponent.Play` (`self.Audio`) 0.0)
      (if (`self.LastCheckpoint`)
        _))))

(fn `UserConstructionScript`)