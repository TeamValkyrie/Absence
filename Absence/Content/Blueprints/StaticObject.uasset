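; StaticObject is an actor with a static mesh that can be switched between hidden and visible in game, with collision following visibility.
; The construction script disables collision when the actor starts hidden and otherwise enables query and physics collision.
; ToggleVisibility flips the hidden state and collision, spawning the PS_SpawningObjects particle effect at the mesh's ParticleEffectSocket when the object reappears.
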(event `self.ReceiveTick`
  (params (DeltaSeconds :type "Float (single-precision)")))

(fn `ToggleVisibility`
  (bind _returnvalue (not (`self.bHidden`)))
  (if _returnvalue
    (`PrimitiveComponent.SetCollisionEnabled` (`self.StaticMesh`) "NoCollision")
    (else
      (`PrimitiveComponent.SetCollisionEnabled` (`self.StaticMesh`) "QueryAndPhysics")
      (`GameplayStatics.SpawnEmitterAtLocation` "/Game/Particles/PS_SpawningObjects.PS_SpawningObjects" (`SceneComponent.GetSocketLocation` (`self.StaticMesh`) "ParticleEffectSocket"))))
  (`self.SetActorHiddenInGame` _returnvalue))

(fn `UserConstructionScript`
  (if (`self.bHidden`)
    (`PrimitiveComponent.SetCollisionEnabled` (`self.StaticMesh`) "NoCollision")
    (else
      (`PrimitiveComponent.SetCollisionEnabled` (`self.StaticMesh`) "QueryAndPhysics"))))