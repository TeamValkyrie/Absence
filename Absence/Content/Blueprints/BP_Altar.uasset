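; Puzzle altar that reacts when a BP_Orb rests on the ground within its sphere, toggling linked objects and altars and optionally teleporting the player or orb to another altar.
; Tick polls the overlap, using flags to fire once, flip static objects (optionally staggered by timers), activate moving objects and spawn particles.
; Orb removal can revert these changes, depending on settings.
; The construction script matches altar collision and overlaps to its hidden state.
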(event `self.ReceiveBeginPlay`)

(event `self.ReceiveTick`
  (params (DeltaSeconds :type "Float (single-precision)"))
  (bind _altartoteleportcharacter (`self.AltarToTeleportCharacter`))
  (bind _sphere (`self.Sphere`))
  (bind _overlappingactors (`PrimitiveComponent.GetOverlappingActors` (`self.Sphere`) "/Game/Blueprints/BP_Orb.BP_Orb_C"))
  ;[1 1 1] IsAltarOverlappingOrb
  (if (>= (`KismetArrayLibrary.Array_LastIndex` _overlappingactors) 0)
    ;[1 1 1] IsOrbNotInHandAndCloseToTheCenterOfAltar
    (bind _asbp_orb (cast `/Game/Blueprints/BP_Orb` (`|GetArrayItem` _overlappingactors)))
    (if (and (`/Game/Blueprints/BP_Orb.OnTheGround` _asbp_orb) (< (`KismetMathLibrary.VSize` (- (`SceneComponent.K2_GetComponentLocation` _sphere) (`SceneComponent.K2_GetComponentLocation` (`/Game/Blueprints/BP_Orb.Sphere` _asbp_orb)))) (`SphereComponent.SphereRadius` _sphere)))
      (`|ExecutionSequence`
        (:`then_0`
          ;[1 1 1] Hide/Show Object if Orb in Altar
          (if (`self.IsTimerSet`)
            (if (not (`self.CanToggleVisibility`))
              (for (_array_element _array_index) (`self.StaticObjects`) :!label _label
                (if (!= (`self.TimeBetweenObjects`) 0.0)
                  (`KismetSystemLibrary.K2_SetTimer` _array_element "ToggleVisibility" (* (`self.TimeBetweenObjects`) (+ (`KismetMathLibrary.Conv_IntToDouble` _array_index) 1e-05)))
                  (else
                    (`KismetSystemLibrary.PrintText` (`KismetTextLibrary.Conv_IntToText` _array_index) false)
                    (bind _returnvalue (not (`Actor.bHidden` _array_element)))
                    (if _returnvalue
                      (`PrimitiveComponent.SetCollisionEnabled` (`/Game/Blueprints/StaticObject.StaticMesh` _array_element) "NoCollision")
                      (else
                        (`PrimitiveComponent.SetCollisionEnabled` (`/Game/Blueprints/StaticObject.StaticMesh` _array_element) "QueryAndPhysics")
                        (`GameplayStatics.SpawnEmitterAtLocation` "/Game/Particles/PS_SpawningObjects.PS_SpawningObjects" (`self.K2_GetActorLocation` _array_element))))
                    (`self.SetActorHiddenInGame` _array_element _returnvalue)))
                (set `self.CanToggleVisibility` true))
              (for _array_element_2 (`self.MovingObjects`)
                (`PrimitiveComponent.SetCollisionEnabled` (`/Game/Blueprints/MovingObjects.StaticMesh` _array_element_2) "QueryAndPhysics")
                (set `/Game/Blueprints/MovingObjects.IsActivated?` true _array_element_2)
                (`self.SetActorHiddenInGame` _array_element_2 false)
                (set `self.CanToggleVisibility` true)
                (if (`/Game/Blueprints/MovingObjects.ObjectNeedsToMoveBack?` _array_element_2)
                  (bind _result (`/Engine/EditorBlueprintResources/StandardMacros.IncrementInt` (`/Game/Blueprints/MovingObjects.TowardPosition` _array_element_2))
                    (:`  `
                      (bind _finaltarget (`/Game/Blueprints/MovingObjects.FinalTarget` _array_element_2))
                      (if (> _result _finaltarget)
                        (set `/Game/Blueprints/MovingObjects.TowardPosition` _finaltarget _array_element_2)))))
                (set `/Game/Blueprints/MovingObjects.ReturnedToStartingPosition` false _array_element_2)
                (`GameplayStatics.SpawnEmitterAtLocation` "/Game/Particles/PS_SpawningObjects.PS_SpawningObjects" (`self.K2_GetActorLocation` _array_element_2)))
              (for _array_element_3 (`self.Altars`)
                (bind _returnvalue_2 (not (`Actor.bHidden` _array_element_3)))
                (if _returnvalue_2
                  (`PrimitiveComponent.SetCollisionEnabled` (`/Game/Blueprints/BP_Altar.SM_altarTree0` _array_element_3) "NoCollision")
                  (set `PrimitiveComponent.bGenerateOverlapEvents` false (`/Game/Blueprints/BP_Altar.Sphere` _array_element_3))
                  (else
                    (`PrimitiveComponent.SetCollisionEnabled` (`/Game/Blueprints/BP_Altar.SM_altarTree0` _array_element_3) "QueryAndPhysics")
                    (bind _sphere_2 (`/Game/Blueprints/BP_Altar.Sphere` _array_element_3))
                    (set `PrimitiveComponent.bGenerateOverlapEvents` true _sphere_2)
                    (`GameplayStatics.SpawnEmitterAtLocation` "/Game/Particles/PS_SpawningObjects.PS_SpawningObjects" (`SceneComponent.K2_GetComponentLocation` _sphere_2))))
                (`self.SetActorHiddenInGame` _array_element_3 _returnvalue_2)
                (set `self.CanToggleVisibility` true)))
            (else
              (`KismetSystemLibrary.K2_SetTimer` null "ToggleVisibility" (`self.Timer`))
              (set `self.IsTimerSet` true)
              (goto _label))))
        (:`then_1`
          ;[1 1 1] Teleport Character
          (if (`self.HasCharacterTeleported`)
            _
            (elif (and (`KismetSystemLibrary.IsValid` (`self.AltarToTeleportCharacter`)) (not (`/Game/Blueprints/BP_Orb.OnAltar` _asbp_orb)))
              (bind _outactors (`GameplayStatics.GetAllActorsOfClass` "/Game/Blueprints/PlayerCharacters/BP_ThirdPersonCharacter.BP_ThirdPersonCharacter_C"))
              (bind _asbp_third_person_character (cast `/Game/Blueprints/PlayerCharacters/BP_ThirdPersonCharacter` (`|GetArrayItem` _outactors)))
              (`self.K2_SetActorLocation` _asbp_third_person_character (+ (`/Game/Blueprints/BP_Altar.SpawnPosition` _altartoteleportcharacter) (`self.K2_GetActorLocation` _altartoteleportcharacter)) false false)
              (set `self.HasCharacterTeleported` true))))
        (:`then_2`
          ;[1 1 1] TeleportOrb
          (if (and (`KismetSystemLibrary.IsValid` (`self.AltarToTeleportOrb`)) (not (`/Game/Blueprints/BP_Orb.OnAltar` _asbp_orb)))
            (`self.K2_SetActorLocation` _asbp_orb (`SceneComponent.K2_GetComponentLocation` (`/Game/Blueprints/BP_Altar.Sphere` (`self.AltarToTeleportOrb`))) false false)
            (set `/Game/Blueprints/BP_Orb.OnAltar` true _asbp_orb))))
      (else
        ;[1 1 1] Hide/Show object when orb is removed from Altar
        (if (and (`self.CanToggleVisibility`) (`self.CanObjectDisappear`)) :!label _label_2
          (if (`self.CanToggleObject`)
            (set `self.CanToggleVisibility` false)
            (else
              (for _array_element_4 (`self.StaticObjects`)
                (`KismetSystemLibrary.K2_ClearTimer` _array_element_4 "ToggleVisibility")
                (if (> (`self.Timer`) 0.0)
                  (`self.SetActorHiddenInGame` _array_element_4 true)
                  (`PrimitiveComponent.SetCollisionEnabled` (`/Game/Blueprints/StaticObject.StaticMesh` _array_element_4) "NoCollision")
                  (set `self.CanToggleVisibility` false)
                  (set `self.HasCharacterTeleported` false)
                  (set `self.IsTimerSet` false)
                  (`KismetSystemLibrary.K2_SetTimer` null "ToggleVisibility")
                  (else
                    (bind _returnvalue_3 (not (`Actor.bHidden` _array_element_4)))
                    (if _returnvalue_3
                      (`PrimitiveComponent.SetCollisionEnabled` (`/Game/Blueprints/StaticObject.StaticMesh` _array_element_4) "NoCollision")
                      (else
                        (`PrimitiveComponent.SetCollisionEnabled` (`/Game/Blueprints/StaticObject.StaticMesh` _array_element_4) "QueryAndPhysics")))
                    (`self.SetActorHiddenInGame` _array_element_4 _returnvalue_3)
                    (set `self.CanToggleVisibility` false)
                    (set `self.HasCharacterTeleported` false)
                    (`KismetSystemLibrary.K2_SetTimer` null "ToggleVisibility")
                    (set `self.IsTimerSet` false))))
              (for _array_element_5 (`self.MovingObjects`)
                (set `/Game/Blueprints/MovingObjects.IsActivated?` false _array_element_5)
                (if (`/Game/Blueprints/MovingObjects.ObjectNeedsToMoveBack?` _array_element_5)
                  (bind _result_2 (`/Engine/EditorBlueprintResources/StandardMacros.DecrementInt` (`/Game/Blueprints/MovingObjects.TowardPosition` _array_element_5))
                    (:`  `
                      (if (< _result_2 0)
                        (set `/Game/Blueprints/MovingObjects.TowardPosition` 0 _array_element_5)))))
                (if (not (`/Game/Blueprints/MovingObjects.ObjectWontChangeVisibility` _array_element_5))
                  (`self.SetActorHiddenInGame` _array_element_5 true)
                  (`PrimitiveComponent.SetCollisionEnabled` (`/Game/Blueprints/MovingObjects.StaticMesh` _array_element_5) "NoCollision"))
                (set `self.CanToggleVisibility` false)
                (set `self.HasCharacterTeleported` false)
                (`KismetSystemLibrary.K2_SetTimer` null "ToggleVisibility")
                (set `self.IsTimerSet` false))
              (for _array_element_6 (`self.Altars`)
                (if (> (`self.Timer`) 0.0)
                  (`self.SetActorHiddenInGame` _array_element_6 (== (`self.Timer`) 0.0))
                  (else
                    (`self.SetActorHiddenInGame` _array_element_6 false)))
                (bind _returnvalue_4 (not (`Actor.bHidden` _array_element_6)))
                (if _returnvalue_4
                  (`PrimitiveComponent.SetCollisionEnabled` (`/Game/Blueprints/BP_Altar.SM_altarTree0` _array_element_6) "NoCollision")
                  (set `PrimitiveComponent.bGenerateOverlapEvents` false (`/Game/Blueprints/BP_Altar.Sphere` _array_element_6))
                  (else
                    (`PrimitiveComponent.SetCollisionEnabled` (`/Game/Blueprints/BP_Altar.SM_altarTree0` _array_element_6) "QueryAndPhysics")
                    (set `PrimitiveComponent.bGenerateOverlapEvents` true (`/Game/Blueprints/BP_Altar.Sphere` _array_element_6))))
                (`self.SetActorHiddenInGame` _array_element_6 _returnvalue_4)
                (set `self.CanToggleVisibility` false)
                (set `self.HasCharacterTeleported` false)
                (`KismetSystemLibrary.K2_SetTimer` null "ToggleVisibility")
                (set `self.IsTimerSet` false))))
          (else
            (set `self.HasCharacterTeleported` false)))))
    (else
      (goto _label_2))))

(fn `ToggleVisibility`
  (for _array_element (`self.StaticObjects`)
    (bind _returnvalue (not (`Actor.bHidden` _array_element)))
    (if _returnvalue
      (`PrimitiveComponent.SetCollisionEnabled` (`/Game/Blueprints/StaticObject.StaticMesh` _array_element) "NoCollision")
      (else
        (`PrimitiveComponent.SetCollisionEnabled` (`/Game/Blueprints/StaticObject.StaticMesh` _array_element) "QueryAndPhysics")))
    (`self.SetActorHiddenInGame` _array_element _returnvalue))
  (for _array_element_2 (`self.MovingObjects`)
    (bind _returnvalue_2 (not (`Actor.bHidden` _array_element_2)))
    (if _returnvalue_2
      (`PrimitiveComponent.SetCollisionEnabled` (`/Game/Blueprints/MovingObjects.StaticMesh` _array_element_2) "NoCollision")
      (else
        (`PrimitiveComponent.SetCollisionEnabled` (`/Game/Blueprints/MovingObjects.StaticMesh` _array_element_2) "QueryAndPhysics")))
    (`self.SetActorHiddenInGame` _array_element_2 _returnvalue_2)))

(fn `UserConstructionScript`
  (bind _output_get (set `PrimitiveComponent.bGenerateOverlapEvents` (not (`self.bHidden`)) (`self.Sphere`)))
  (if _output_get
    (`PrimitiveComponent.SetCollisionEnabled` (`self.SM_altarTree0`) "QueryAndPhysics")
    (else
      (`PrimitiveComponent.SetCollisionEnabled` (`self.SM_altarTree0`) "NoCollision"))))