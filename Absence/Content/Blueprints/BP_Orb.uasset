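; Carryable glowing orb that the player picks up into the lantern, drops with physics or sets on a BP_Altar.
; Tick polls click or E with a short cooldown, lerps the carried orb to the lantern socket and respawns it below a death height.
; Sphere handles pickup, altar detection and a gate.
; Sphere1 overlap flags make Tick fade the darkness post-process through a material parameter collection near the orb.
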(event `self.Sphere.OnComponentBeginOverlap`
  (params (OverlappedComponent :type "PrimitiveComponent Object Reference") (OtherActor :type "Actor Object Reference") (OtherComp :type "PrimitiveComponent Object Reference") (OtherBodyIndex :type Integer) (bFromSweep :type Boolean) (SweepResult :type "HitResult Structure (by ref)"))
  (if (`self.OnTheGround`)
    (`/Engine/EditorBlueprintResources/StandardMacros.Gate` true :!via `Open` :!label _label)))

(event `self.Sphere.OnComponentEndOverlap`
  (params (OverlappedComponent :type "PrimitiveComponent Object Reference") (OtherActor :type "Actor Object Reference") (OtherComp :type "PrimitiveComponent Object Reference") (OtherBodyIndex :type Integer))
  (goto _label :!via `Close`))

(event `self.ReceiveBeginPlay`
  ;[1 1 1] Set initial transform
  (set `self.InitialPosition` (`self.K2_GetActorLocation`))
  (set `self.InitialRotation` (`KismetMathLibrary.Conv_RotatorToVector` (`self.K2_GetActorRotation`)))
  (`AudioComponent.Play` (`self.orbGlow_loop_Cue`) 0.0))

(event `self.ReceiveTick`
  (params (DeltaSeconds :type "Float (single-precision)"))
  (bind _returnvalue (`GameplayStatics.GetPlayerController` 0))
  (bind (_returnvalue_x _returnvalue_y _returnvalue_z) (`KismetMathLibrary.BreakVector` (`self.K2_GetActorLocation`)))
  (bind _staticmesh (`self.StaticMesh`))
  (bind _overlappingactors (`PrimitiveComponent.GetOverlappingActors` (`self.Sphere`) "/Game/Blueprints/BP_Altar.BP_Altar_C"))
  (set `self.Timer` (- (`self.Timer`) (`GameplayStatics.GetWorldDeltaSeconds`)))
  (if (> _returnvalue_z (`self.DeathValueZ`))
    (if (`self.Switch`)
      (`self.Overlap_True`)
      (else
        (`self.Overlap_False`)))
    (if (`self.OnAltar`)
      (bind _asbp_altar (cast `/Game/Blueprints/BP_Altar` (`|GetArrayItem` (`PrimitiveComponent.GetOverlappingActors` (`self.Sphere`) "/Game/Blueprints/BP_Altar.BP_Altar_C"))))
      (`self.K2_SetActorLocation` (`SceneComponent.K2_GetComponentLocation` (`/Game/Blueprints/BP_Altar.Sphere` _asbp_altar)) false true))
    (if (`self.OnTheGround`)
      (if (>= (`KismetArrayLibrary.Array_LastIndex` (`PrimitiveComponent.GetOverlappingActors` (`self.Sphere`) "/Game/Blueprints/PlayerCharacters/BP_ThirdPersonCharacter.BP_ThirdPersonCharacter_C")) 0)
        (bind _asbp_third_person_character (cast `/Game/Blueprints/PlayerCharacters/BP_ThirdPersonCharacter` (`GameplayStatics.GetPlayerCharacter` 0)))
        (if (and (not (`/Game/Blueprints/PlayerCharacters/BP_ThirdPersonCharacter.PlayerHasAlreadyAnOrb` _asbp_third_person_character)) (or (`PlayerController.IsInputKeyDown` (`GameplayStatics.GetPlayerController` 0) "LeftMouseButton") (`PlayerController.IsInputKeyDown` (`GameplayStatics.GetPlayerController` 0) "E")) (<= (`self.Timer`) 0.0))
          (set `self.Timer` 0.2)
          (`AudioComponent.Stop` (`self.orbGlow_loop_Cue`))
          (`GameplayStatics.SpawnSoundAttached` "/Game/Audio/Actions/orbPickup_Cue.orbPickup_Cue" (`self.Sphere`) "None" (0.0 0.0 0.0) (struct) "KeepRelativeOffset" false 0.8 1.0 0.0 null null)
          (set `self.OnTheGround` false)
          (`PrimitiveComponent.SetSimulatePhysics` (`self.StaticMesh`) false)
          (set `self.OnAltar` false)
          (set `/Game/Blueprints/PlayerCharacters/BP_ThirdPersonCharacter.PlayerHasAlreadyAnOrb` true _asbp_third_person_character)
          (`SceneComponent.SetWorldScale3D` (`self.StaticMesh`) (0.01 0.01 0.01))
          (`SceneComponent.SetRelativeScale3D` (`self.Orb_Effect_01`) (125.0 125.0 125.0))
          (`SceneComponent.SetRelativeScale3D` (`self.Orb_Effect_02`) (125.0 125.0 125.0))
          (`ActorComponent.SetActive` (`self.Sphere1`) false false)))
      (elif (and (or (`PlayerController.IsInputKeyDown` _returnvalue "LeftMouseButton") (`PlayerController.IsInputKeyDown` _returnvalue "E")) (<= (`self.Timer`) 0.0))
        (set `self.Timer` 0.2)
        (`AudioComponent.Play` (`self.orbGlow_loop_Cue`) 0.0)
        (if (>= (`KismetArrayLibrary.Array_LastIndex` _overlappingactors) 0)
          (bind _asbp_altar_2 (cast `/Game/Blueprints/BP_Altar` (`|GetArrayItem` _overlappingactors)))
          (`self.K2_SetActorLocation` (`SceneComponent.K2_GetComponentLocation` (`/Game/Blueprints/BP_Altar.Sphere` _asbp_altar_2)) false true)
          (`PrimitiveComponent.SetSimulatePhysics` (`self.StaticMesh`) false)
          (set `self.OnAltar` true)
          (`GameplayStatics.SpawnSoundAttached` "/Game/Audio/Actions/orbActivation_Cue.orbActivation_Cue" (`self.Sphere`) "None" (0.0 0.0 0.0) (struct) "KeepRelativeOffset" false 0.8 1.0 0.0 null null)
          (else
            (`PrimitiveComponent.SetSimulatePhysics` (`self.StaticMesh`) true)))
        (set `self.OnTheGround` true)
        (bind _asbp_third_person_character_2 (cast `/Game/Blueprints/PlayerCharacters/BP_ThirdPersonCharacter` (`GameplayStatics.GetPlayerCharacter` 0)))
        (set `/Game/Blueprints/PlayerCharacters/BP_ThirdPersonCharacter.PlayerHasAlreadyAnOrb` false _asbp_third_person_character_2)
        (`SceneComponent.SetWorldScale3D` (`self.StaticMesh`) (0.125 0.125 0.125))
        (`SceneComponent.SetRelativeScale3D` (`self.Orb_Effect_01`) (75.0 75.0 75.0))
        (`SceneComponent.SetRelativeScale3D` (`self.Orb_Effect_02`) (75.0 75.0 75.0))
        (`ActorComponent.SetActive` (`self.Sphere1`) true true)
        (else
          (bind _asbp_third_person_character_3 (cast `/Game/Blueprints/PlayerCharacters/BP_ThirdPersonCharacter` (`GameplayStatics.GetPlayerCharacter` 0)))
          (bind _lantern (`/Game/Blueprints/PlayerCharacters/BP_ThirdPersonCharacter.Lantern` _asbp_third_person_character_3))
          (`self.K2_SetActorLocationAndRotation` (`KismetMathLibrary.VLerp` (`SceneComponent.K2_GetComponentLocation` _staticmesh) (- (`SceneComponent.GetSocketLocation` _lantern "LanternSocket") (* (`KismetMathLibrary.GetUpVector` (`SceneComponent.GetSocketRotation` _lantern "LanternSocket")) (`.SphereRadius` (`KismetSystemLibrary.GetComponentBounds` _staticmesh)))) 0.9) (`SceneComponent.GetSocketRotation` _lantern "LanternSocket")))))
    (else
      (`self.Respawn`))))

(event `self.Sphere1.OnComponentBeginOverlap`
  (params (OverlappedComponent :type "PrimitiveComponent Object Reference") (OtherActor :type "Actor Object Reference") (OtherComp :type "PrimitiveComponent Object Reference") (OtherBodyIndex :type Integer) (bFromSweep :type Boolean) (SweepResult :type "HitResult Structure (by ref)"))
  ;[1 1 1] Orb effect
  (if (or (`ActorComponent.ComponentHasTag` OtherComp "CameraCollision") (== (`GameplayStatics.GetObjectClass` OtherActor) "/Game/Blueprints/PlayerCharacters/BP_ThirdPersonCharacter.BP_ThirdPersonCharacter_C"))
    (set `self.Switch` true)))

(event `Overlap_True`
  ;[1 1 1] Orb effect
  (bind _returnvalue (`KismetMaterialLibrary.GetScalarParameterValue` "/Game/FX/M_darknessPP3_Collection.M_darknessPP3_Collection" "BlendWeight"))
  (`KismetMaterialLibrary.SetScalarParameterValue` "/Game/FX/M_darknessPP3_Collection.M_darknessPP3_Collection" "BlendWeight" (`KismetMathLibrary.FInterpTo` _returnvalue 0.0 (`GameplayStatics.GetWorldDeltaSeconds`) 3.5)))

(event `self.Sphere1.OnComponentEndOverlap`
  (params (OverlappedComponent :type "PrimitiveComponent Object Reference") (OtherActor :type "Actor Object Reference") (OtherComp :type "PrimitiveComponent Object Reference") (OtherBodyIndex :type Integer))
  ;[1 1 1] Orb effect
  (if (or (== (`GameplayStatics.GetObjectClass` OtherActor) "/Game/Blueprints/PlayerCharacters/BP_ThirdPersonCharacter.BP_ThirdPersonCharacter_C") (`ActorComponent.ComponentHasTag` OverlappedComponent "CameraCollision"))
    (set `self.Switch` false)))

(event `Overlap_False`
  ;[1 1 1] Orb effect
  (bind _returnvalue (`KismetMaterialLibrary.GetScalarParameterValue` "/Game/FX/M_darknessPP3_Collection.M_darknessPP3_Collection" "BlendWeight"))
  (`KismetMaterialLibrary.SetScalarParameterValue` "/Game/FX/M_darknessPP3_Collection.M_darknessPP3_Collection" "BlendWeight" (`KismetMathLibrary.FInterpTo` _returnvalue 1.0 (`GameplayStatics.GetWorldDeltaSeconds`) 3.5)))

(event `Respawn`
  ;[1 1 1] Orb respawning
  (`GameplayStatics.PlaySound2D` "/Game/Audio/Actions/orbPickup_Cue.orbPickup_Cue" 1.0 1.0 0.0 null null)
  (`PrimitiveComponent.SetSimulatePhysics` (`self.StaticMesh`) true)
  (set `self.OnTheGround` true)
  (bind _asbp_third_person_character (cast `/Game/Blueprints/PlayerCharacters/BP_ThirdPersonCharacter` (`GameplayStatics.GetPlayerCharacter` 0)))
  (set `/Game/Blueprints/PlayerCharacters/BP_ThirdPersonCharacter.PlayerHasAlreadyAnOrb` false _asbp_third_person_character)
  (`SceneComponent.SetWorldScale3D` (`self.StaticMesh`) (0.125 0.125 0.125))
  (`SceneComponent.SetRelativeScale3D` (`self.Orb_Effect_01`) (75.0 75.0 75.0))
  (`SceneComponent.SetRelativeScale3D` (`self.Orb_Effect_02`) (75.0 75.0 75.0))
  (`ActorComponent.SetActive` (`self.Sphere1`) true true)
  (`self.K2_SetActorLocationAndRotation` (`self.InitialPosition`) (`KismetMathLibrary.Conv_VectorToRotator` (`self.InitialRotation`))))

(fn `UserConstructionScript`)