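; Follow camera that tracks the third-person character along one world axis selected by AxisToLock.
; BeginPlay caches the first BP_ThirdPersonCharacter found in the level as PlayerRef.
; Each Tick copies that character's mesh coordinate on the chosen axis to the Camera, leaving the other two unchanged, with no smoothing.
; With no axis chosen, the camera stays put and only a log message is printed.
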(event `self.ReceiveBeginPlay`
  ;[1 1 1] Init
  (bind _outactors (`GameplayStatics.GetAllActorsOfClass` "/Game/Blueprints/PlayerCharacters/BP_ThirdPersonCharacter.BP_ThirdPersonCharacter_C"))
  (bind _output_get (set `self.PlayerRef` (`|GetArrayItem` _outactors)))
  (`KismetSystemLibrary.PrintString` (`KismetSystemLibrary.GetDisplayName` _output_get) false))

(event `self.ReceiveTick`
  (params (DeltaSeconds :type "Float (single-precision)"))
  (bind _camera (`self.Camera`))
  (bind (_returnvalue_x _returnvalue_y _returnvalue_z) (`KismetMathLibrary.BreakVector` (`SceneComponent.K2_GetComponentLocation` (`self.Camera`))))
  (bind (_returnvalue_x_2 _returnvalue_y_2 _returnvalue_z_2) (`KismetMathLibrary.BreakVector` (`SceneComponent.K2_GetComponentLocation` (`Character.Mesh` (`self.PlayerRef`)))))
  ;[1 1 1] Update Position
  (switch `string` (`self.AxisToLock`)
    (:`Default`
      ;[1 1 1] Print when no Axis is selected
      (`KismetSystemLibrary.PrintString` "No Axis chosen" false true (struct :`G` 0.66 :`B` 1.0 :`A` 1.0) (`GameplayStatics.GetWorldDeltaSeconds`)))
    (:`X`
      (`SceneComponent.K2_SetWorldLocation` _camera (`KismetMathLibrary.MakeVector` _returnvalue_x_2 _returnvalue_y _returnvalue_z) false false))
    (:`Y`
      (`SceneComponent.K2_SetWorldLocation` _camera (`KismetMathLibrary.MakeVector` _returnvalue_x _returnvalue_y_2 _returnvalue_z) false false))
    (:`Z`
      (`SceneComponent.K2_SetWorldLocation` _camera (`KismetMathLibrary.MakeVector` _returnvalue_x _returnvalue_y _returnvalue_z_2) false false))))

(fn `UserConstructionScript`)