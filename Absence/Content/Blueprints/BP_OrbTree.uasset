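; Orb tree actor that holds a fake orb, which the player turns into a real BP_Orb.
; Sphere1 overlaps with the character or camera collision toggle a switch that Tick uses to interpolate the darkness collection's BlendWeight toward 0 inside, 1 outside.
; Tick also polls left mouse while the pawn is in Sphere, then once destroys the fake orb, light, meshes, post-process and Sphere1 and spawns BP_Orb there.
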(event `self.ReceiveTick`
  (params (DeltaSeconds :type "Float (single-precision)"))
  (bind _returnvalue (`GameplayStatics.GetPlayerController` 0))
  ;[1 1 1] Overlap Check
  (if (`self.Switch`)
    (`self.Overlap_True`)
    (else
      (`self.Overlap_False`)))
  ;[1 1 1] Check if player is in radius and is pressing left mouse button
  (if (and (`PlayerController.IsInputKeyDown` _returnvalue "LeftMouseButton") (`PrimitiveComponent.IsOverlappingActor` (`self.Sphere`) (`Controller.K2_GetPawn` _returnvalue)))
    ;[1 1 1] Remove old Orb and Spawn Real orb
    (`/Engine/EditorBlueprintResources/StandardMacros.DoOnce` false
      (:`Completed`
        (bind _output_get (set `self.SpawnLocation` (`SceneComponent.K2_GetComponentToWorld` (`self.FakeOrb`))))
        (`ActorComponent.K2_DestroyComponent` (`self.PointLight`))
        (`ActorComponent.K2_DestroyComponent` (`self.FakeOrb`))
        (`ActorComponent.K2_DestroyComponent` (`self.StaticMesh1`))
        (`ActorComponent.K2_DestroyComponent` (`self.StaticMesh`))
        (`ActorComponent.K2_DestroyComponent` (`self.PostProcess`))
        (`ActorComponent.K2_DestroyComponent` (`self.Sphere1`))
        (`|SpawnActorFromClass` "/Game/Blueprints/BP_Orb.BP_Orb_C" _output_get "Undefined" "OverrideRootScale" null null)))))

(event `self.Sphere1.OnComponentBeginOverlap`
  (params (OverlappedComponent :type "PrimitiveComponent Object Reference") (OtherActor :type "Actor Object Reference") (OtherComp :type "PrimitiveComponent Object Reference") (OtherBodyIndex :type Integer) (bFromSweep :type Boolean) (SweepResult :type "HitResult Structure (by ref)"))
  ;[1 1 1] Orb effect
  (if (or (`ActorComponent.ComponentHasTag` OtherComp "CameraCollision") (== (`GameplayStatics.GetObjectClass` OtherActor) "/Game/Blueprints/PlayerCharacters/BP_ThirdPersonCharacter.BP_ThirdPersonCharacter_C"))
    (set `self.Switch` true)))

(event `Overlap_True`
  ;[1 1 1] Orb effect
  (bind _returnvalue (`KismetMaterialLibrary.GetScalarParameterValue` "/Game/FX/M_darknessPP3_Collection.M_darknessPP3_Collection" "BlendWeight"))
  (`KismetMaterialLibrary.SetScalarParameterValue` "/Game/FX/M_darknessPP3_Collection.M_darknessPP3_Collection" "BlendWeight" (`KismetMathLibrary.FInterpTo` _returnvalue 0.0 (`GameplayStatics.GetWorldDeltaSeconds`) 3.5)))

(event `self.Sphere1.OnComponentEndOverlap`
  (params (OverlappedComponent :type "PrimitiveComponent Object Reference") (OtherActor :type "Actor Object Reference") (OtherComp :type "PrimitiveComponent Object Reference") (OtherBodyIndex :type Integer))
  ;[1 1 1] Orb effect
  (if (or (== (`GameplayStatics.GetObjectClass` OtherActor) "/Game/Blueprints/PlayerCharacters/BP_ThirdPersonCharacter.BP_ThirdPersonCharacter_C") (`ActorComponent.ComponentHasTag` OverlappedComponent "CameraCollision"))
    (set `self.Switch` false)))

(event `Overlap_False`
  ;[1 1 1] Orb effect
  (bind _returnvalue (`KismetMaterialLibrary.GetScalarParameterValue` "/Game/FX/M_darknessPP3_Collection.M_darknessPP3_Collection" "BlendWeight"))
  (`KismetMaterialLibrary.SetScalarParameterValue` "/Game/FX/M_darknessPP3_Collection.M_darknessPP3_Collection" "BlendWeight" (`KismetMathLibrary.FInterpTo` _returnvalue 1.0 (`GameplayStatics.GetWorldDeltaSeconds`) 3.5)))

(fn `UserConstructionScript`)