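; On-rails camera actor that glides through a stored list of transforms, optionally looping back to the first.
; Tick interpolates toward the current transform with TInterpTo, dividing default speed by that point's multiplier, so higher values move slower.
; Near arrival within tolerance, NextLocation advances the index; the Moving flag is set but never read here.
; Editor utility events append the camera's current transform or snap the actor to the first.
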(event `self.ReceiveBeginPlay`
  ;[1 1 1] Are we at the last slide?
  (if (== (`self.CurrentLocation`) (- (`KismetArrayLibrary.Array_Length` (`self.CameraLocations`)) 1)) :!label _label
    (if (`self.Loop`)
      ;[1 1 1] If true, let's return to the first one
      (set `self.CurrentLocation` 0)
      (set `self.Moving` true))
    (else
      ;[1 1 1] If false, let's keep moving
      (set `self.CurrentLocation` (+ (`self.CurrentLocation`) 1))
      (set `self.Moving` true))))

(event `NextLocation`
  ;[1 1 1] Are we at the last slide?
  (goto _label))

(event `self.ReceiveTick`
  (params (DeltaSeconds :type "Float (single-precision)"))
  (bind _output (`|GetArrayItem` (`self.CameraLocations`) (`self.CurrentLocation`)))
  ;[1 1 1] Event Tick
  ;[1 1 1] TInterpt to new position
  (`self.K2_SetActorTransform` (`KismetMathLibrary.TInterpTo` (`self.GetTransform`) _output (`GameplayStatics.GetWorldDeltaSeconds`) (/ (`self.DefaultSpeed`) (`|GetArrayItem` (`self.CameraLocationsMoveSpeedMultiplier`) (`self.CurrentLocation`)))))
  ;[1 1 1] When we are almost there, let's go to the next location
  (if (`KismetMathLibrary.NearlyEqual_TransformTransform` _output (`self.GetTransform`) 40.0 5.0 0.1)
    (`self.NextLocation`)))

(event `AddCurrentPosition`
  (bind _cameralocationsmovespeedmultiplier (`self.CameraLocationsMoveSpeedMultiplier`))
  (bind _cameralocations (`self.CameraLocations`))
  ;[1 1 1] Blutility
  ;;[1 1 1] Add the Current position to the camera slides
  (`KismetArrayLibrary.Array_Set` _cameralocations (`KismetArrayLibrary.Array_Length` _cameralocations) (`SceneComponent.K2_GetComponentToWorld` (`self.Camera`)) true)
  ;;[1 1 1] Add a default speed
  (`KismetArrayLibrary.Array_Set` _cameralocationsmovespeedmultiplier (`KismetArrayLibrary.Array_Length` _cameralocationsmovespeedmultiplier) 1.0 true))

(event `SetCameraToFirstPosition`
  ;[1 1 1] Blutility
  (`self.K2_SetActorTransform` (`|GetArrayItem` (`self.CameraLocations`))))

(fn `UserConstructionScript`)