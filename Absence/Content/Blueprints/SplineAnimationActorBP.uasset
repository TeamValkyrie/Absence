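; Actor that moves a skeletal mesh along its spline component over time.
; Tick accumulates elapsed seconds in CurrentDistance, scales it by MovementSpeed as a fraction of spline length, and sets the mesh's world transform there, with no looping.
; Roll and pitch come only from the spline's start, while yaw stays the mesh's own and scale follows the actor.
; A Movement node is left unconnected.
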(event `self.ReceiveBeginPlay`)

(event `self.ReceiveTick`
  (params (DeltaSeconds :type "Float (single-precision)"))
  (bind _spline (`self.Spline`))
  (bind (_returnvalue_roll _returnvalue_pitch) (`KismetMathLibrary.BreakRotator` (`SplineComponent.GetRotationAtDistanceAlongSpline` _spline 0.0 "World")))
  (bind (_returnvalue_roll_2 _returnvalue_pitch_2 _returnvalue_yaw) (`KismetMathLibrary.BreakRotator` (`SceneComponent.K2_GetComponentRotation` (`self.SkeletalMesh`))))
  (bind _output_get (set `self.CurrentDistance` (+ DeltaSeconds (`self.CurrentDistance`))))
  (`SceneComponent.K2_SetWorldTransform` (`self.SkeletalMesh`) (`KismetMathLibrary.MakeTransform` (`SplineComponent.GetLocationAtDistanceAlongSpline` _spline (* (`SplineComponent.GetSplineLength` _spline) (* _output_get (`self.MovementSpeed`))) "World") (`KismetMathLibrary.MakeRotator` _returnvalue_roll _returnvalue_pitch _returnvalue_yaw) (`self.GetActorScale3D`)) false false))

(fn `UserConstructionScript`)