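; Moving object actor that, while activated, either travels through a list of target points or orbits a pivot point around yaw, optionally stopping at a target or swinging back.
; BeginPlay converts locally authored points to world space, and Tick drives the motion with timer-delayed waypoint advances, looping or stopping at FinalTarget.
; When deactivated, it can retrace waypoints, rotate back or head straight to start, snapping there if hidden.
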(event `self.ReceiveBeginPlay`
  (bind _staticmesh (`self.StaticMesh`))
  (set `self.StartingPosition` (`SceneComponent.K2_GetComponentLocation` _staticmesh))
  (set `self.StartingRotation` (`SceneComponent.K2_GetComponentRotation` _staticmesh))
  (set `self.RotationPosition` (`KismetMathLibrary.TransformLocation` (`self.GetTransform`) (* (`self.RotationPosition`) 1.0)))
  (for (_array_element _array_index) (`self.PositionTargets`)
    (`KismetArrayLibrary.Array_Set` (`self.PositionTargets`) _array_index (`KismetMathLibrary.TransformLocation` (`self.GetTransform`) _array_element)))
  (set `self.ObjectMustStopAtTarget?` (!= (`self.RotationTarget`) (0.0 0.0 0.0)))
  (set `self.RotationTarget` (`KismetMathLibrary.TransformLocation` (`self.GetTransform`) (`self.RotationTarget`))))

(event `self.ReceiveTick`
  (params (DeltaSeconds :type "Float (single-precision)"))
  (bind (_returnvalue_roll _returnvalue_pitch _returnvalue_yaw) (`KismetMathLibrary.BreakRotator` (`self.K2_GetActorRotation`)))
  (bind _returnvalue (`self.K2_GetActorLocation`))
  (bind (_returnvalue_roll_2 _returnvalue_pitch_2 _returnvalue_yaw_2) (`KismetMathLibrary.BreakRotator` (`self.K2_GetActorRotation`)))
  (bind _returnvalue_2 (`self.K2_GetActorLocation`))
  (bind (_returnvalue_roll_3 _returnvalue_pitch_3 _returnvalue_yaw_3) (`KismetMathLibrary.BreakRotator` (`self.K2_GetActorRotation`)))
  (bind _returnvalue_3 (`self.K2_GetActorLocation`))
  (bind (_returnvalue_roll_4 _returnvalue_pitch_4 _returnvalue_yaw_4) (`KismetMathLibrary.BreakRotator` (`self.K2_GetActorRotation`)))
  (bind (_returnvalue_roll_5 _returnvalue_pitch_5 _returnvalue_yaw_5) (`KismetMathLibrary.BreakRotator` (`self.K2_GetActorRotation`)))
  (bind _rotationposition (`self.RotationPosition`))
  (bind _rotationposition_2 (`self.RotationPosition`))
  (bind _rotationposition_3 (`self.RotationPosition`))
  (bind _rotationposition_4 (`self.RotationPosition`))
  (bind _rotationposition_5 (`self.RotationPosition`))
  (bind _output (`|GetArrayItem` (`self.PositionTargets`) (`self.TowardPosition`)))
  (bind (_returnvalue_x _returnvalue_y _returnvalue_z) (`KismetMathLibrary.BreakVector` (- (`KismetMathLibrary.MakeVector` _returnvalue_roll_3 _returnvalue_pitch_3 _returnvalue_yaw_3) (* (`KismetMathLibrary.MakeVector` 0.0 0.0 (`self.RotationSpeed`)) (`GameplayStatics.GetWorldDeltaSeconds`)))))
  (bind (_returnvalue_x_2 _returnvalue_y_2 _returnvalue_z_2) (`KismetMathLibrary.BreakVector` (- (`KismetMathLibrary.MakeVector` _returnvalue_roll_4 _returnvalue_pitch_4 _returnvalue_yaw_4) (* (`KismetMathLibrary.MakeVector` 0.0 0.0 (`self.RotationSpeed`)) (`GameplayStatics.GetWorldDeltaSeconds`)))))
  (bind (_returnvalue_x_3 _returnvalue_y_3 _returnvalue_z_3) (`KismetMathLibrary.BreakVector` (+ (`KismetMathLibrary.MakeVector` _returnvalue_roll _returnvalue_pitch _returnvalue_yaw) (* (`KismetMathLibrary.MakeVector` 0.0 0.0 (`self.RotationSpeed`)) (`GameplayStatics.GetWorldDeltaSeconds`)))))
  (bind (_returnvalue_x_4 _returnvalue_y_4 _returnvalue_z_4) (`KismetMathLibrary.BreakVector` (+ (`KismetMathLibrary.MakeVector` _returnvalue_roll_2 _returnvalue_pitch_2 _returnvalue_yaw_2) (* (`KismetMathLibrary.MakeVector` 0.0 0.0 (`self.RotationSpeed`)) (`GameplayStatics.GetWorldDeltaSeconds`)))))
  (bind (_returnvalue_x_5 _returnvalue_y_5 _returnvalue_z_5) (`KismetMathLibrary.BreakVector` (+ (`KismetMathLibrary.MakeVector` _returnvalue_roll_5 _returnvalue_pitch_5 _returnvalue_yaw_5) (* (`KismetMathLibrary.MakeVector` 0.0 0.0 (`self.RotationSpeed`)) (`GameplayStatics.GetWorldDeltaSeconds`)))))
  (if (`self.IsActivated?`)
    (if (>= (`KismetArrayLibrary.Array_LastIndex` (`self.PositionTargets`)) 0)
      (if (not (and (> (`self.TowardPosition`) (`self.FinalTarget`)) (> (`self.FinalTarget`) 0)))
        (if (`self.CanMove`)
          (if (<= (`KismetMathLibrary.VSize` (- (`self.K2_GetActorLocation`) (`|GetArrayItem` (`self.PositionTargets`) (`self.TowardPosition`)))) 10.0)
            (if (<= (`KismetSystemLibrary.K2_GetTimerRemainingTime` null "MoveToNextTarget") 0.0)
              (`KismetSystemLibrary.K2_SetTimer` null "MoveToNextTarget" (+ (`self.Timer`) 1e-06))
              (set `self.CanMove` false))
            (else
              (`self.K2_SetActorLocation` (+ _returnvalue_2 (* (* (`KismetMathLibrary.GetDirectionUnitVector` _returnvalue_2 (`|GetArrayItem` (`self.PositionTargets`) (`self.TowardPosition`))) (`self.Speed`)) (`GameplayStatics.GetWorldDeltaSeconds`))))))))
      (elif (not (== (`self.RotationPosition`) (`KismetMathLibrary.MakeVector` 0.0)))
        (set `self.IsRotating?` true)
        (if (`self.ObjectMustStopAtTarget?`)
          (if (not (`self.CanRotateBetweenPoints?`))
            (if (> (`KismetMathLibrary.VSize` (- (`self.RotationTarget`) (`self.K2_GetActorLocation`))) (`self.OffsetFromRotationTarget`))
              (`self.K2_SetActorLocationAndRotation` (+ _rotationposition_3 (* (`KismetMathLibrary.GetForwardVector` (`KismetMathLibrary.MakeRotator` _returnvalue_x_5 _returnvalue_y_5 _returnvalue_z_5)) (`KismetMathLibrary.VSize` (- _rotationposition_3 (`self.K2_GetActorLocation`))))) (`KismetMathLibrary.MakeRotator` _returnvalue_x_5 _returnvalue_y_5 _returnvalue_z_5)))
            (elif (not (`self.MustMoveToStartingPosition`))
              (if (> (`KismetMathLibrary.VSize` (- (`self.RotationTarget`) (`self.K2_GetActorLocation`))) (`self.OffsetFromRotationTarget`))
                (`self.K2_SetActorLocationAndRotation` (+ _rotationposition_4 (* (`KismetMathLibrary.GetForwardVector` (`KismetMathLibrary.MakeRotator` _returnvalue_x_3 _returnvalue_y_3 _returnvalue_z_3)) (`KismetMathLibrary.VSize` (- _rotationposition_4 (`self.K2_GetActorLocation`))))) (`KismetMathLibrary.MakeRotator` _returnvalue_x_3 _returnvalue_y_3 _returnvalue_z_3))
                (else
                  (set `self.MustMoveToStartingPosition` true)))
              (elif (> (`KismetMathLibrary.VSize` (- (`self.StartingPosition`) (`self.K2_GetActorLocation`))) (`self.OffsetFromRotationTarget`))
                (`self.K2_SetActorLocationAndRotation` (+ _rotationposition_2 (* (`KismetMathLibrary.GetForwardVector` (`KismetMathLibrary.MakeRotator` _returnvalue_x_2 _returnvalue_y_2 _returnvalue_z_2)) (`KismetMathLibrary.VSize` (- _rotationposition_2 (`self.K2_GetActorLocation`))))) (`KismetMathLibrary.MakeRotator` _returnvalue_x_2 _returnvalue_y_2 _returnvalue_z_2)))))
          (else
            (`self.K2_SetActorLocationAndRotation` (+ _rotationposition_5 (* (`KismetMathLibrary.GetForwardVector` (`KismetMathLibrary.MakeRotator` _returnvalue_x_4 _returnvalue_y_4 _returnvalue_z_4)) (`KismetMathLibrary.VSize` (- _rotationposition_5 (`self.K2_GetActorLocation`))))) (`KismetMathLibrary.MakeRotator` _returnvalue_x_4 _returnvalue_y_4 _returnvalue_z_4))))))
    (elif (`self.ObjectNeedsToMoveBack?`)
      (if (not (`self.bHidden`))
        (if (`self.ObjectNeedsToMoveBackwardFromPointToPoint?`)
          (if (and (`self.CanMove`) (not (`self.ReturnedToStartingPosition`)))
            (`self.K2_SetActorLocation` (+ _returnvalue (* (* (`KismetMathLibrary.GetDirectionUnitVector` _returnvalue _output) (`self.Speed`)) (`GameplayStatics.GetWorldDeltaSeconds`))))
            (if (<= (`KismetMathLibrary.VSize` (- (`self.K2_GetActorLocation`) _output)) 10.0)
              (if (<= (`KismetSystemLibrary.K2_GetTimerRemainingTime` null "MoveToPreviousTarget") 0.0)
                (`KismetSystemLibrary.K2_SetTimer` null "MoveToPreviousTarget" 1e-06)
                (set `self.CanMove` false))))
          (elif (`self.IsRotating?`)
            (if (> (`KismetMathLibrary.VSize` (- (`self.StartingPosition`) (`self.K2_GetActorLocation`))) (`self.OffsetFromRotationTarget`))
              (`self.K2_SetActorLocationAndRotation` (+ _rotationposition (* (`KismetMathLibrary.GetForwardVector` (`KismetMathLibrary.MakeRotator` _returnvalue_x _returnvalue_y _returnvalue_z)) (`KismetMathLibrary.VSize` (- _rotationposition (`self.K2_GetActorLocation`))))) (`KismetMathLibrary.MakeRotator` _returnvalue_x _returnvalue_y _returnvalue_z)))
            (else
              (`self.K2_SetActorLocation` (+ _returnvalue_3 (* (* (`KismetMathLibrary.GetDirectionUnitVector` _returnvalue_3 (`self.StartingPosition`)) (`self.Speed`)) (`GameplayStatics.GetWorldDeltaSeconds`)))))))
        (else
          (set `self.TowardPosition` 0)
          (`self.K2_SetActorLocationAndRotation` (`self.StartingPosition`) (`self.StartingRotation`))
          (set `self.CanMove` true))))))

(fn `MoveToNextTarget`
  (bind _finaltarget (`self.FinalTarget`))
  (set `self.ReturnedToStartingPosition` false)
  (`/Engine/EditorBlueprintResources/StandardMacros.IncrementInt` (`self.TowardPosition`)
    (:`  `
      (set `self.CanMove` true)
      (if (> (`self.TowardPosition`) (`KismetArrayLibrary.Array_LastIndex` (`self.PositionTargets`)))
        (set `self.TowardPosition` 0)
        (elif (and (> (`self.TowardPosition`) _finaltarget) (> _finaltarget 0))
          (set `self.TowardPosition` (`self.FinalTarget`)))))))

(fn `MoveToPreviousTarget`
  (`/Engine/EditorBlueprintResources/StandardMacros.DecrementInt` (`self.TowardPosition`)
    (:`  `
      (set `self.CanMove` true)
      (if (< (`self.TowardPosition`) 0)
        (set `self.TowardPosition` 0)
        (set `self.ReturnedToStartingPosition` true)
        (else
          (set `self.ReturnedToStartingPosition` false))))))

(fn `UserConstructionScript`
  (bind _returnvalue (`KismetMathLibrary.TransformLocation` (`self.GetTransform`) (`self.RotationPosition`)))
  (if (`self.bHidden`)
    (`PrimitiveComponent.SetCollisionEnabled` (`self.StaticMesh`) "NoCollision")
    (else
      (`PrimitiveComponent.SetCollisionEnabled` (`self.StaticMesh`) "QueryAndPhysics")))
  (`KismetSystemLibrary.PrintText` "Platform-PivotPoint Distance:" false)
  (`KismetSystemLibrary.PrintText` (`KismetTextLibrary.Conv_DoubleToText` (`KismetMathLibrary.VSize` (- _returnvalue (`self.K2_GetActorLocation`))) "HalfToEven") false)
  (`KismetSystemLibrary.PrintText` "Target-PivotPoint distance:" false)
  (`KismetSystemLibrary.PrintText` (`KismetTextLibrary.Conv_DoubleToText` (`KismetMathLibrary.VSize` (- _returnvalue (`KismetMathLibrary.TransformLocation` (`self.GetTransform`) (`self.RotationTarget`)))) "HalfToEven") false))